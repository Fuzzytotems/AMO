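; Spell effect for the friendly variant of the Druid's Hibernate, which temporarily alters the owning player's cooldown dilation.
; BeginPlay raises CdDilation on the owner's BP_ArenaPlayerState, and Dispel subtracts the same amount before running the parent dispel.
; The OnEffect override, which receives instigator, amount, damage type and victim, dispels the effect whenever it fires, after calling the parent.
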(event `self.ReceiveBeginPlay`
  (`parent.ReceiveBeginPlay`)
  (bind _asarena_character (cast `/Game/ArenaAssets/ArenaCharacter` (`self.GetOwner`)))
  (bind _asbp_arena_player_state (cast `/Game/ArenaAssets/BP_ArenaPlayerState` (`Pawn.PlayerState` _asarena_character)))
  (set `ArenaPlayerState.cdDilation` (+ (`ArenaPlayerState.cdDilation` _asbp_arena_player_state) 2.0) _asbp_arena_player_state))

(event `self.Dispel`
  (bind _asarena_character (cast `/Game/ArenaAssets/ArenaCharacter` (`self.GetOwner`)))
  (bind _asbp_arena_player_state (cast `/Game/ArenaAssets/BP_ArenaPlayerState` (`Pawn.PlayerState` _asarena_character)))
  (set `ArenaPlayerState.cdDilation` (- (`ArenaPlayerState.cdDilation` _asbp_arena_player_state) 2.0) _asbp_arena_player_state)
  (`parent.Dispel`))

(fn `OnEffect`
  (params (Instigator :type "/Game/ArenaAssets/ArenaCharacter Object Reference") (Amount :type "Float (double-precision)") (DamageType :type "/Game/ArenaAssets/EDamageTypes Enum" :default "NewEnumerator0") (Victim :type "/Game/ArenaAssets/ArenaCharacter Object Reference"))
  (returns (NewDamageAmount :type "Float (double-precision)"))
  (bind _newdamageamount (`parent.OnEffect` Instigator Amount DamageType Victim))
  (`self.Dispel`)
  (return _newdamageamount))

(fn `UserConstructionScript`
  (`parent.UserConstructionScript`))