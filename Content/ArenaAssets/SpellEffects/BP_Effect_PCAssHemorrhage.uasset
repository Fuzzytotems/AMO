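; Spell effect Blueprint for Hemorrhage that applies the BP_Effect_PCAssHemoStatus effect to its owning arena character.
; The OnEffect override casts the owner to ArenaCharacter, applies the status with this effect's instigator as source, and returns Amount unchanged.
; The diminished-effect modifier multiplies HemoConstant by zero, and BeginPlay and construction only call the parent.
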(event `self.ReceiveBeginPlay`
  (`parent.ReceiveBeginPlay`))

(event `self.ReceiveActorBeginOverlap`
  (params (OtherActor :type "Actor Object Reference")))

(event `self.ReceiveTick`
  (params (DeltaSeconds :type "Float (single-precision)")))

(fn `OnEffect`
  (params (Instigator :type "/Game/ArenaAssets/ArenaCharacter Object Reference") (Amount :type "Float (double-precision)") (DamageType :type "/Game/ArenaAssets/EDamageTypes Enum" :default "NewEnumerator0") (Victim :type "/Game/ArenaAssets/ArenaCharacter Object Reference"))
  (returns (NewDamageAmount :type "Float (double-precision)"))
  (bind _asarena_character (cast `/Game/ArenaAssets/ArenaCharacter` (`self.GetOwner`)))
  (`/Game/ArenaAssets/ArenaCharacter.ApplyEffect` _asarena_character "/Game/ArenaAssets/SpellEffects/BP_Effect_PCAssHemoStatus.BP_Effect_PCAssHemoStatus_C" 0 (* 0.0 (`self.HemoConstant`)) (cast `/Game/ArenaAssets/ArenaCharacter` (`self.GetInstigator`) :!pure true))
  (return Amount))

(fn `UserConstructionScript`
  (`parent.UserConstructionScript`))