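; Spell effect actor for the player Cleric's bouncing heal, judging by its name, built on a parent effect class.
; On each effect it computes an effectiveness value from its damage range and applies it to the victim through the server damage handler with the incoming damage type.
; It then re-enables AOELogic before running the parent effect.
; Parent destruction handling runs only when no ticks remain.
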(event `self.ReceiveBeginPlay`
  (`parent.ReceiveBeginPlay`))

(event `self.ReceiveActorBeginOverlap`
  (params (OtherActor :type "Actor Object Reference")))

(event `self.ReceiveTick`
  (params (DeltaSeconds :type "Float (single-precision)")))

(event `self.ReceiveDestroyed`
  (if (not (> (`self.TicksRemaining`) 0.0))
    (`parent.ReceiveDestroyed`)))

(fn `OnEffect`
  (params (Instigator :type "/Game/ArenaAssets/ArenaCharacter Object Reference") (Amount :type "Float (double-precision)") (DamageType :type "/Game/ArenaAssets/EDamageTypes Enum" :default "NewEnumerator0") (Victim :type "/Game/ArenaAssets/ArenaCharacter Object Reference"))
  (returns (NewDamageAmount :type "Float (double-precision)"))
  (`self.RetrieveDamageRange`)
  (bind _damage (`self.CalculateEffectiveness`))
  (`/Game/ArenaAssets/ArenaCharacter.HandleDamage_Server` Victim _damage (`self.DamageType`) (`Pawn.GetController` Instigator) self false false)
  (`/Game/ArenaAssets/Spells/BP_SpellLogic.Reenable` (`self.AOELogic`))
  (bind _newdamageamount (`parent.OnEffect` Instigator Amount DamageType Victim))
  (return _newdamageamount))

(fn `UserConstructionScript`
  (`parent.UserConstructionScript`))