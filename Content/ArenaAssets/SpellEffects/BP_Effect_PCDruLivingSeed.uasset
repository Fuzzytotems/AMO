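; Spell effect Blueprint for the player Druid's Living Seed, which procs on an ArenaCharacter owner until that character reaches full health.
; BeginPlay subtracts the default stack count from the tick count, then zeroes the stacks.
; Each proc at full health re-enables the AOE logic and dispels the effect.
; Otherwise, the diminished-effect modifier is seeded if zero or compounded slightly upward.
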(event `self.ReceiveBeginPlay`
  (set `self.Ticks` (- (`self.Ticks`) (`KismetMathLibrary.Conv_IntToDouble` (`self.DefaultStacks`))))
  (set `self.DefaultStacks` 0)
  (`parent.ReceiveBeginPlay`))

(event `self.ProcActivation`
  (bind _diminishedeffectmodifier (`self.DiminishedEffectModifier`))
  (`parent.ProcActivation`)
  (bind _asarena_character (cast `/Game/ArenaAssets/ArenaCharacter` (`self.GetOwner`)))
  (if (>= (`/Game/ArenaAssets/ArenaCharacter.GetHPPercentage` _asarena_character) 1.0)
    (`/Game/ArenaAssets/Spells/BP_SpellLogic.Reenable` (`self.AOELogic`))
    (`self.Dispel`)
    (elif (== _diminishedeffectmodifier 0.0)
      (set `self.DiminishedEffectModifier` 0.05)
      (else
        (set `self.DiminishedEffectModifier` (* _diminishedeffectmodifier 1.02))))))

(event `self.ReceiveDestroyed`)

(fn `UserConstructionScript`
  (`parent.UserConstructionScript`))