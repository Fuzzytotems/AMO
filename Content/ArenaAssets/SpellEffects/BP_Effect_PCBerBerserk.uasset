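; Berserk spell effect that boosts its owner's outgoing damage of one type while draining the owner's resource.
; On BeginPlay it adds a damage modifier scaled by the diminished-effect modifier, then zeroes that value before running the parent logic.
; Each proc activation removes a fixed amount of resource, and when the owner has less than that amount it still drains, then dispels itself.
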(event `self.ReceiveBeginPlay`
  (`KismetArrayLibrary.Array_Add` (`self.DamageModifiers`) (make `/Game/ArenaAssets/DamageModifierStruct` "NewEnumerator20" (* (`self.DiminishedEffectModifier`) 2.0)))
  (set `self.DiminishedEffectModifier` 0.0)
  (`parent.ReceiveBeginPlay`))

(event `self.ProcActivation`
  (bind _asarena_character (cast `/Game/ArenaAssets/ArenaCharacter` (`self.GetOwner`) :!pure true))
  (`parent.ProcActivation`)
  (if (>= (`ArenaMastersOnlineCharacter.currentResource` _asarena_character) 10.0)
    (`/Game/ArenaAssets/ArenaCharacter.AddExcessResource` _asarena_character -10.0 :!label _label)
    (else
      (`|ExecutionSequence`
        (:`then_0`
          (goto _label))
        (:`then_1`
          (`self.Dispel`))))))

(fn `UserConstructionScript`
  (`parent.UserConstructionScript`))