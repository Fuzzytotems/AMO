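; Spellbook owned by an ArenaCharacter, handling server-side targeting and cast requests for spells defined in a data table.
; Targeting branches on aiming type; frame targeting applies faction rules, with self and target-of-target fallbacks.
; Cast requests check school lockouts and resource, then set IsCasting, whose OnRep informs the character.
; Validity confirmation always passes; mana cost handling is unfinished, and non-frame aiming simply forwards the current target.
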(event Custom|LocalRequestCastSpell
  (params (SpellIndex :type Name) (New%20Target :type Actor%20Object%20Reference) (New%20Mouse%20Hit%20Result :type Hit%20Result%20Structure))
  (if (not (Variables|Default|GetbIsCasting))
    (CallFunction|RequestCastSpellServer SpellIndex New%20Target New%20Mouse%20Hit%20Result)))

(event Custom|HandleTargeting_Local
  (params (SpellIndex :type Name))
  (CallFunction|CheckSpellValidityServer SpellIndex))

(event Custom|HandleTargeting_Server
  (params (SpellIndex :type Name))
  (bind _returnvalue (Components|GetOwner))
  (bind _asarena_character (Utilities|Casting|CastToArenaCharacter _returnvalue))
  (bind _returnvalue_2 (Utilities|GetDataTableRow "/Game/ArenaAssets/SpellTable.SpellTable" SpellIndex)
    (:then
      (switch Utilities|FlowControl|Switch|SwitchonEAimingType (.AimingType (Utilities|Struct|BreakBP_SpellStruct _returnvalue_2))
        (:AT_FrameTarget
          (CallFunction|FrameTargeting (.PlayerTargetingRules (Utilities|Struct|BreakBP_SpellStruct _returnvalue_2))))
        (:AT_SkillShot
          (Default|HandleTargetingSuccessful _asarena_character (Variables|Default|GetTarget) :!label _label))
        (:AT_AutoTarget
          (goto _label))
        (:AT_Toggled
          (goto _label))
        (:AT_GroundTargeted
          (Variables|/Game/ArenaAssets/ArenaCharacter.ArenaCharacter_C|SetWaitingForTarget _asarena_character true)
          (goto _label))))))

(event Custom|RequestCastSpell_Server
  (params (SpellIndex :type Name) (New%20Target :type Actor%20Object%20Reference) (New%20Mouse%20Hit%20Result :type Hit%20Result%20Structure))
  (Networking|SwitchHasAuthority
    (:Authority
      (if (not (Variables|Default|GetbIsCasting))
        (CallFunction|RequestCastSpellFnc SpellIndex New%20Target New%20Mouse%20Hit%20Result)))))

(event Custom|CheckSpellValidity_Server
  (params (SpellIndex :type Name))
  (bind _isvalid (CallFunction|ConfirmSpellValidity SpellIndex))
  (if _isvalid
    (CallFunction|HandleTargetingServer SpellIndex)))

(event EventBeginPlay)

(event Collision|EventActorBeginOverlap
  (params (OtherActor :type Actor%20Object%20Reference)))

(event EventTick
  (params (DeltaSeconds :type Float%20%28single-precision%29))
  (Networking|SwitchHasAuthority))

(fn ConstructionScript
  (bind _asarena_character (Utilities|Casting|CastToArenaCharacter (Components|GetOwner)))
  (Variables|/Game/ArenaAssets/ArenaCharacter.ArenaCharacter_C|SetbIsCasting _asarena_character (Variables|Default|GetbIsCasting)))

(fn RequestCastSpellFnc
  (params (SpellDataName :type Name) (NewTarget :type Actor%20Object%20Reference) (NewMouseHitResult :type Hit%20Result%20Structure))
  (bind _returnvalue (Utilities|GetDataTableRow "/Game/ArenaAssets/SpellTable.SpellTable" SpellDataName)
    (:then
      (bind _array_element (Utilities|Array|ForEachLoopwithBreak (Variables|Default|GetLockouts) :!label _label)
        (:LoopBody
          (if (not (== (Utilities|Array|FindItem (.MagicSchools (Utilities|Struct|BreakBP_SpellStruct _returnvalue)) (.School (Utilities|Struct|BreakLockoutStruct _array_element))) -1))
            (LocalVariables|SetResult false)
            (goto _label Break)))
        (:Completed
          (Variables|Default|SetSpellIndex SpellDataName)
          (bind _returnvalue_2 (Utilities|GetDataTableRow "/Game/ArenaAssets/SpellTable.SpellTable" (Variables|Default|GetSpellIndex))
            (:then
              (if (>= (Variables|/Script/ArenaMastersOnline.ArenaMastersOnlineCharacter|GetcurrentResource (.AsArena%20Character (Utilities|Casting|CastToArenaCharacter (Components|GetOwner)))) (.BaseResourceCost (Utilities|Struct|BreakBP_SpellStruct _returnvalue_2)))
                _
                (else
                  (LocalVariables|SetResult false)))
              (Variables|Default|SetbIsCasting (LocalVariables|GetResult)))))))))

(fn OnRepBIsCasting
  (bind _biscasting (Variables|Default|GetbIsCasting))
  (bind _spellindex (Variables|Default|GetSpellIndex))
  (bind _asarena_character (Utilities|Casting|CastToArenaCharacter (Components|GetOwner)))
  (if (not (Math|Boolean|Equal(Boolean) _biscasting (Variables|/Game/ArenaAssets/ArenaCharacter.ArenaCharacter_C|GetbIsCasting _asarena_character)))
    (bind _returnvalue (Utilities|GetDataTableRow "/Game/ArenaAssets/SpellTable.SpellTable" _spellindex)
      (:then
        (Default|ChangeIsCastingLocal _asarena_character _biscasting _spellindex)))))

(fn ConfirmSpellValidity
  (params (SpellIndex :type Name))
  (return true))

(fn InvalidTarget
  (bind _asarena_character (Utilities|Casting|CastToArenaCharacter (Components|GetOwner)))
  (Default|InvalidTarget _asarena_character))

(fn FrameTargeting
  (params (PlayerTargetingRules :type PlayerTargetingRules%20Enum))
  (bind _returnvalue (Components|GetOwner))
  (bind _returnvalue_2 (Components|GetOwner))
  (bind _asarena_character (Utilities|Casting|CastToArenaCharacter _returnvalue))
  (bind _asarena_character_2 (Utilities|Casting|CastToArenaCharacter _returnvalue_2))
  ;[1 1 1] Begin by checking if the player has a targe.t  If the player does not, the player should only be able to cast self-targeted, either-targeted, or friendly targeted spells.  If the player has a target,
  ; some smart targeting mechanisms are in place.
  (Utilities|IsValid (Variables|Default|GetTarget)
    (:Is%20Valid
      (switch Utilities|FlowControl|Switch|SwitchonPlayerTargetingRules PlayerTargetingRules
        (:NewEnumerator3
          (if (== (Variables|/Game/ArenaAssets/ArenaCharacter.ArenaCharacter_C|GetFaction _asarena_character_2) (Variables|/Game/ArenaAssets/ArenaCharacter.ArenaCharacter_C|GetFaction (Variables|Default|GetTarget)))
            (if (== (Variables|/Game/ArenaAssets/ArenaCharacter.ArenaCharacter_C|GetFaction (.AsArena%20Character (Utilities|Casting|CastToArenaCharacter (Variables|/Script/ArenaMastersOnline.ArenaMastersOnlineCharacter|GetTarget (Variables|Default|GetTarget))))) (Variables|/Game/ArenaAssets/ArenaCharacter.ArenaCharacter_C|GetFaction (.AsArena%20Character (Utilities|Casting|CastToArenaCharacter (Components|GetOwner)))))
              (Variables|Default|SetTarget (.AsArena%20Character (Utilities|Casting|CastToArenaCharacter (Variables|/Script/ArenaMastersOnline.ArenaMastersOnlineCharacter|GetTarget (Variables|Default|GetTarget)))) :!label _label)))
          (Default|HandleTargetingSuccessful _asarena_character_2 (Variables|Default|GetTarget) :!label _label_2))
        (:NewEnumerator1
          (if (== (Variables|/Game/ArenaAssets/ArenaCharacter.ArenaCharacter_C|GetFaction _asarena_character_2) (Variables|/Game/ArenaAssets/ArenaCharacter.ArenaCharacter_C|GetFaction (Variables|Default|GetTarget))) :!label _label_3
            (goto _label_2)
            (elif (== (Variables|/Game/ArenaAssets/ArenaCharacter.ArenaCharacter_C|GetFaction (.AsArena%20Character (Utilities|Casting|CastToArenaCharacter (Variables|/Script/ArenaMastersOnline.ArenaMastersOnlineCharacter|GetTarget (Variables|Default|GetTarget))))) (Variables|/Game/ArenaAssets/ArenaCharacter.ArenaCharacter_C|GetFaction (.AsArena%20Character (Utilities|Casting|CastToArenaCharacter (Components|GetOwner)))))
              (goto _label)
              (else
                (CallFunction|InvalidTarget :!label _label_4)))))
        (:NewEnumerator2
          (if (== (Variables|Default|GetTarget) _asarena_character)
            (goto _label_4)
            (else
              (goto _label_3))))
        (:NewEnumerator0
          (Variables|Default|SetTarget _asarena_character :!label _label_5)
          (goto _label_2))
        (:NewEnumerator4
          (goto _label_2))))
    (:Is%20Not%20Valid
      (switch Utilities|FlowControl|Switch|SwitchonPlayerTargetingRules PlayerTargetingRules
        (:NewEnumerator3
          (goto _label_4))
        (:NewEnumerator1
          (goto _label_5))
        (:NewEnumerator2
          (goto _label_4))
        (:NewEnumerator0
          (goto _label_5))
        (:NewEnumerator4
          (goto _label_5))))))

(fn SkillShotTargeting
  (params (PlayerTargetingRules :type PlayerTargetingRules%20Enum))
  (Default|HandleTargetingSuccessful (.AsArena%20Character (Utilities|Casting|CastToArenaCharacter (Components|GetOwner))) (Variables|Default|GetTarget)))

(fn HandleManaCost
  (params (BeforeCast :type Boolean))
  (bind _returnvalue (Utilities|GetDataTableRow "/Game/ArenaAssets/SpellTable.SpellTable" (Variables|Default|GetSpellIndex))
    (:then
      (switch Utilities|FlowControl|Switch|SwitchonECastingType (.CastingType (Utilities|Struct|BreakBP_SpellStruct _returnvalue))))))