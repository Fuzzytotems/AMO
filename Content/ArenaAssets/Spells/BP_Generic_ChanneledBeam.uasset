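; Channeled beam spell actor that links its instigator to a homing target, damaging that target on each pulse.
; BeginPlay feeds both actors to the particle system as beam source and target parameters, then runs the parent logic.
; Each ActivatePulse deals calculated damage through HandleDamageServer and applies the PCCleAegis effect to the same target, with starting stacks derived from half of SpecialDamageVar, truncated.
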(event `self.ReceiveBeginPlay`
  (bind _particlesystem (`self.ParticleSystem`))
  (`ParticleSystemComponent.SetActorParameter` _particlesystem "TargetActor" (`self.HomingTarget`))
  (`ParticleSystemComponent.SetActorParameter` _particlesystem "SourceActor" (`self.GetInstigator`))
  (`parent.ReceiveBeginPlay`))

(event `self.ActivatePulse`
  (bind _totaldamage (`self.CalculateDamage`))
  (`/Game/ArenaAssets/ArenaCharacter.HandleDamage_Server` (`self.HomingTarget`) _totaldamage (`self.DamageType`) (`self.GetInstigatorController`) self false false)
  (`/Game/ArenaAssets/ArenaCharacter.ApplyEffect` (`self.HomingTarget`) "/Game/ArenaAssets/SpellEffects/BP_Effect_PCCleAegis.BP_Effect_PCCleAegis_C" (`KismetMathLibrary.FTrunc` (/ (`self.SpecialDamageVar`) 2.0)) 0.0 (cast `/Game/ArenaAssets/ArenaCharacter` (`self.Instigator`) :!pure true) null))

(fn `UserConstructionScript`
  (`parent.UserConstructionScript`))