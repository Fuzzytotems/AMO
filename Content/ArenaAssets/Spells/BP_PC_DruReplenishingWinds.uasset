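; Druid Replenishing Winds spell actor that applies its replenishing effect to a group of friendly characters in a single pulse.
; On BeginPlay it attaches to the homing target, or to the owner pawn without one, then pulses after a tiny delay.
; The pulse affects a friendly homing target first, then the leading entries of the sorted Friendlies array, taking one fewer when that target received it.
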(event `self.ReceiveBeginPlay`
  (bind _homingtarget (`self.HomingTarget`))
  (`self.K2_AttachRootComponentToActor` (select `bool` (`KismetSystemLibrary.IsValid` _homingtarget) :`false` (`self.OwnerPawn`) :`true` _homingtarget :!type "Actor Object Reference") "None" "SnapToTarget")
  (`parent.ReceiveBeginPlay`)
  (`KismetSystemLibrary.Delay` 0.01)
  (`self.ActivatePulse`))

(event `self.ActivatePulse`
  (bind _homingtarget (`self.HomingTarget`))
  (bind (_success _friendly) (`self.IsFriendly` _homingtarget))
  (bind _returnvalue (and _friendly _success))
  (if _returnvalue
    (`/Game/ArenaAssets/ArenaCharacter.ApplyEffect` _homingtarget "/Game/ArenaAssets/SpellEffects/BP_Effect_PCDruReplenishingWinds.BP_Effect_PCDruReplenishingWinds_C" 0 0.0 (`self.OwnerPawn`) self)
    (`/Game/ArenaAssets/ArenaCharacter.ApplyEffect` (`self.HomingTarget`) "/Game/ArenaAssets/SpellEffects/BP_Effect_PCDruReplenishingWinds.BP_Effect_PCDruReplenishingWinds_C" 0 0.0 (`self.OwnerPawn`) self))
  (bind _output (`FuzzytotemsAugmenterBPLibrary.TArraySortObject` (`self.Friendlies`) "EST_Sort"))
  (for _index (range (+ (select `bool` _returnvalue :`false` 5 :`true` 4) 1))
    (bind _asarena_character (cast `/Game/ArenaAssets/ArenaCharacter` (`KismetArrayLibrary.Array_Get` _output _index)))
    (`/Game/ArenaAssets/ArenaCharacter.ApplyEffect` _asarena_character "/Game/ArenaAssets/SpellEffects/BP_Effect_PCDruReplenishingWinds.BP_Effect_PCDruReplenishingWinds_C" 0 0.0 (`self.OwnerPawn`) self)))

(fn `UserConstructionScript`
  (`parent.UserConstructionScript`))