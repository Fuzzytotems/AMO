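; PC_Tranquility is a pulsing spell actor for Tranquility that applies its effect to arena characters in an area.
; On each server pulse activation, it gathers every ArenaCharacter overlapping its Sphere and applies SpellEffect to each, crediting the spell's instigator.
; The Blueprint only defines this pulse response; the pulse trigger, sphere setup and effect contents are not defined in its graphs.
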(event `self.ReceiveBeginPlay`
  (`parent.ReceiveBeginPlay`))

(event `self.ActivatePulse_Server`
  (for _array_element (`PrimitiveComponent.GetOverlappingActors` (`self.Sphere`) "/Game/ArenaAssets/ArenaCharacter.ArenaCharacter_C")
    (bind _asarena_character (cast `/Game/ArenaAssets/ArenaCharacter` _array_element))
    (`/Game/ArenaAssets/ArenaCharacter.ApplyEffect` _asarena_character "/Game/ArenaAssets/SpellEffects/SpellEffect.SpellEffect_C" (cast `/Game/ArenaAssets/ArenaCharacter` (`self.Instigator`) :!pure true) 0.0)))

(fn `UserConstructionScript`
  (`parent.UserConstructionScript`))