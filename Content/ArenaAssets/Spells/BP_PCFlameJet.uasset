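; BP_PCFlameJet is a flame jet spell actor that deals area damage to enemies in pulses.
; On BeginPlay it assigns its capsule as the AOE collision volume, runs the parent setup, then snaps itself onto its instigator.
; Each ActivatePulse loops over the Enemies array, calculates damage per target and applies it through ArenaCharacter's HandleDamageServer, crediting the instigator's controller.
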(event `self.ReceiveBeginPlay`
  (set `self.AOECollisionVolume` (`self.Capsule`))
  (`parent.ReceiveBeginPlay`)
  (`self.K2_AttachRootComponentToActor` (`self.GetInstigator`) "None" "SnapToTarget"))

(event `self.ActivatePulse`
  (for _array_element (`self.Enemies`)
    (bind _totaldamage (`self.CalculateDamage`))
    (`/Game/ArenaAssets/ArenaCharacter.HandleDamage_Server` (cast `/Game/ArenaAssets/ArenaCharacter` _array_element :!pure true) _totaldamage (`self.DamageType`) (`self.GetInstigatorController`) self)))

(fn `UserConstructionScript`
  (`parent.UserConstructionScript`))