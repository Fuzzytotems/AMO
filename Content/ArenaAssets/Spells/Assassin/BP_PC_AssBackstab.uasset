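; BP_PC_AssBackstab is the Assassin's backstab spell actor, which rewards striking a target from behind.
; On BeginPlay it takes the dot product of the owning ArenaCharacter's and HomingTarget's forward vectors to judge positioning.
; Closer alignment sets a higher ChargePercentile and grants the owner more ExcessResource, in three tiers.
; It then calls the parent BeginPlay, which receives the adjusted charge.
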(event `self.ReceiveBeginPlay`
  (bind _asarena_character (cast `/Game/ArenaAssets/ArenaCharacter` (`self.GetOwner`) :!pure true))
  (bind _excessresource (`ArenaMastersOnlineCharacter.excessResource` _asarena_character))
  (bind _returnvalue (`KismetMathLibrary.Dot_VectorVector` (`KismetMathLibrary.Conv_RotatorToVector` (`self.K2_GetActorRotation` _asarena_character)) (`KismetMathLibrary.Conv_RotatorToVector` (`self.K2_GetActorRotation` (`self.HomingTarget`)))))
  (`|ExecutionSequence`
    (:`then_0`
      (if (> _returnvalue 0.65)
        (set `self.ChargePercentile` 4.0)
        (set `ArenaMastersOnlineCharacter.excessResource` (+ _excessresource 15.0) _asarena_character)
        (elif (> _returnvalue 0.0)
          (set `self.ChargePercentile` 2.0)
          (set `ArenaMastersOnlineCharacter.excessResource` (+ _excessresource 5.0) _asarena_character)
          (else
            (set `self.ChargePercentile` 1.0)))))
    (:`then_1`
      (`parent.ReceiveBeginPlay`))))

(event `self.ReceiveActorBeginOverlap`
  (params (OtherActor :type "Actor Object Reference")))

(event `self.ReceiveTick`
  (params (DeltaSeconds :type "Float (single-precision)")))

(fn `UserConstructionScript`
  (`parent.UserConstructionScript`))