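; Assassin Pommel Strike spell actor that attempts a timed lockout on its homing target as soon as it spawns.
; When the lockout succeeds, it grants excess resource to the owning ArenaCharacter and modifies Pommel Strike's own cooldown through that character's player state.
; All logic runs once in BeginPlay after the parent call, with no tick or overlap handling.
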(event `self.ReceiveBeginPlay`
  (bind _asarena_character (cast `/Game/ArenaAssets/ArenaCharacter` (`self.GetOwner`) :!pure true))
  (`parent.ReceiveBeginPlay`)
  (bind _result (`/Game/ArenaAssets/ArenaCharacter.AttemptLockout_Fnc` (`self.HomingTarget`) 4.0))
  (if _result
    (`/Game/ArenaAssets/ArenaCharacter.AddExcessResource` _asarena_character 10.0)
    (`ArenaPlayerState.ModifySpecificCD` (cast `/Game/ArenaAssets/BP_ArenaPlayerState` (`Pawn.PlayerState` _asarena_character) :!pure true) "PC_AssPommelStrike" 15.0)))

(event `self.ReceiveActorBeginOverlap`
  (params (OtherActor :type "Actor Object Reference")))

(event `self.ReceiveTick`
  (params (DeltaSeconds :type "Float (single-precision)")))

(fn `UserConstructionScript`
  (`parent.UserConstructionScript`))