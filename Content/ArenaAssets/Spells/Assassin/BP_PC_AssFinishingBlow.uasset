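; Assassin Finishing Blow spell Blueprint that hits harder the lower the homing target's health is.
; On BeginPlay, it divides the resource spent by a dampener, then a math expression scales that momentum up to fourfold as target HP falls toward zero.
; The result is stored as ChargePercentile before the parent BeginPlay runs, leaving the rest of the spell's behavior to the parent class.
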(event EventBeginPlay
  (Variables|Default|SetChargePercentile (|(MomentumDamage*(1+(3*(1-HPPerc)))) (/ (Math|Conversions|ToFloat(Integer) (.ResourceSpent (Utilities|Struct|BreakSpellInfoStruct (Variables|Default|GetStatStruct)))) (Variables|Default|GetConstantDampener)) (Default|GetHPPercentage (Variables|Default|GetHomingTarget))))
  (|CallParentFunction))

(fn ConstructionScript
  (|CallParentFunction))