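; Cleric splash heal spell actor that applies its effect to one secondary friendly besides the homing target.
; After the parent BeginPlay and a brief delay, it sorts the Friendlies array and picks the first entry that is not the HomingTarget.
; That character receives the CalculateDamage result through HandleDamageServer, credited to the instigator's controller, and the loop stops there.
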(event `self.ReceiveBeginPlay`
  (`parent.ReceiveBeginPlay`)
  (`KismetSystemLibrary.Delay` 0.01)
  (bind _output (`FuzzytotemsAugmenterBPLibrary.TArraySortObject` (`self.Friendlies`) "EST_Sort"))
  (for _array_element _output
    (if (!= _array_element (`self.HomingTarget`))
      (bind _totaldamage (`self.CalculateDamage`))
      (`/Game/ArenaAssets/ArenaCharacter.HandleDamage_Server` (cast `/Game/ArenaAssets/ArenaCharacter` _array_element :!pure true) _totaldamage "NewEnumerator0" (`Pawn.GetController` (`self.Instigator`)) self false false)
      (break))))

(fn `UserConstructionScript`
  (`parent.UserConstructionScript`))