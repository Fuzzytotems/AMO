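; Cleric spell actor for Prayer of Shielding, which grants the Aegis effect to friendly characters.
; On BeginPlay it teleports to its homing target, runs the parent logic, then fires a pulse after a very short delay.
; The pulse gives each friendly Aegis stacks equal to the truncated calculated damage value, credited to the instigator.
; Handling for more than six friendlies is unimplemented and only prints a placeholder.
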(event `self.ReceiveBeginPlay`
  (`self.K2_SetActorLocation` (`self.K2_GetActorLocation` (`self.HomingTarget`)) false true)
  (`parent.ReceiveBeginPlay`)
  (`KismetSystemLibrary.Delay` 0.01)
  (`self.ActivatePulse`))

(event `self.ActivatePulse`
  (bind _friendlies (`self.Friendlies`))
  (if (> (`KismetArrayLibrary.Array_Length` _friendlies) 6)
    ;[1 0 0.1341] TODO: > 6 Players Logic
    (`KismetSystemLibrary.PrintString` "NYI")
    (else
      (for _array_element _friendlies
        (bind _asarena_character (cast `/Game/ArenaAssets/ArenaCharacter` _array_element))
        (bind _totaldamage (`self.CalculateDamage`))
        (`/Game/ArenaAssets/ArenaCharacter.ApplyEffect` _asarena_character "/Game/ArenaAssets/SpellEffects/BP_Effect_PCCleAegis.BP_Effect_PCCleAegis_C" (`KismetMathLibrary.FTrunc` _totaldamage) 0.0 (cast `/Game/ArenaAssets/ArenaCharacter` (`self.Instigator`) :!pure true) null)))))

(fn `UserConstructionScript`
  (`parent.UserConstructionScript`))