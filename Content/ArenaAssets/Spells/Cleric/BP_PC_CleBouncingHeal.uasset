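; Cleric bouncing heal spell: a homing projectile that applies a heal effect to successive friendly targets.
; On server-side overlap with its homing target, it applies the effect, hides, disables collision and spends an activation.
; Reenable retargets to the first sorted friendly, or the second if that is the current target, then restores the projectile.
; It destroys itself when activations run out or no alternate target exists.
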(event `self.ReceiveBeginPlay`
  (set `self.AOECollisionVolume` (`self.BounceRadius`))
  (`parent.ReceiveBeginPlay`))

(event `self.ProjectileSphere.OnComponentBeginOverlap`
  (params (OtherActor :type "Actor Object Reference") (OtherComp :type "PrimitiveComponent Object Reference") (OtherBodyIndex :type Integer) (bFromSweep :type Boolean) (SweepResult :type "HitResult Structure (by ref)"))
  (bind _homingtarget (`self.HomingTarget`))
  (cast `/Game/ArenaAssets/ArenaCharacter` OtherActor)
  (`/Engine/EditorBlueprintResources/StandardMacros.DoOnce` false :!label _label
    (:`Completed`
      (`/Engine/EditorBlueprintResources/ActorMacros.Switch Has Authority`
        (:`Authority`
          (if (== OtherActor _homingtarget)
            (`/Game/ArenaAssets/ArenaCharacter.ApplyEffect` _homingtarget "/Game/ArenaAssets/SpellEffects/BP_Effect_PCCleBouncingHeal.BP_Effect_PCCleBouncingHeal_C" 0 0.0 (cast `/Game/ArenaAssets/ArenaCharacter` (`self.Instigator`) :!pure true) self)
            (`self.Disable`)
            (else
              (goto _label :!via `Reset`))))
        (:`Remote`
          (goto _label :!via `Reset`))))))

(event `self.Reenable`
  (`|ExecutionSequence`
    (:`then_0`
      (bind _output (`FuzzytotemsAugmenterBPLibrary.TArraySortObject` (`self.Friendlies`) "EST_UnstableSort"))
      (bind _item (`KismetArrayLibrary.Array_Get` _output))
      (if (!= _item (`self.HomingTarget`))
        (bind _output_get (set `self.HomingTarget` (cast `/Game/ArenaAssets/ArenaCharacter` _item :!pure true)))
        (`self.Set Homing Target` _output_get :!label _label_2)
        (`self.SetActorHiddenInGame` false)
        (`PrimitiveComponent.SetCollisionEnabled` (`self.ProjectileSphere`) "QueryOnly")
        (else
          (bind _item_2 (`KismetArrayLibrary.Array_Get` _output 1))
          (bind (_asarena_character _bsuccess) (cast `/Game/ArenaAssets/ArenaCharacter` _item_2 :!pure true))
          (if (and (`KismetSystemLibrary.IsValid` _item_2) _bsuccess)
            (set `self.HomingTarget` _asarena_character)
            (goto _label_2)
            (else
              (`self.DestroyLogic`))))))
    (:`then_1`
      (goto _label :!via `Reset`))))

(event `self.Disable`
  (`self.SetActorHiddenInGame` true)
  (`PrimitiveComponent.SetCollisionEnabled` (`self.ProjectileSphere`) "NoCollision")
  (bind _output_get (set `self.ActivationsRemaining` (- (`self.ActivationsRemaining`) 1)))
  (if (<= _output_get 0)
    (`self.DestroyLogic`)))

(fn `UserConstructionScript`
  (`parent.UserConstructionScript`))