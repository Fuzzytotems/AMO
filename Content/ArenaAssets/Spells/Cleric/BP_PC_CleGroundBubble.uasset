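; BP_PC_CleGroundBubble is a Cleric spell actor that creates a ground area bubble with a damage absorption pool.
; On the server, it applies the AOE bubble effect to characters entering the overlap and dispels it when they leave.
; The pool is set from CalculateDamage shortly after BeginPlay.
; HandleDamage drains that shared pool, returns any unabsorbed damage, and destroys the spell logic once the pool is empty.
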(event EventBeginPlay
  (|CallParentFunction)
  (Utilities|FlowControl|Delay 0.01)
  (bind _totaldamage (CallFunction|CalculateDamage))
  (Variables|Default|SetSpecialDamageVar _totaldamage))

(event EventActorBeginOverlap
  (params (OtherActor :type Actor%20Object%20Reference))
  (Networking|SwitchHasAuthority
    (:Authority
      (bind _asarena_character (Utilities|Casting|CastToArenaCharacter OtherActor))
      (Default|ApplyEffect _asarena_character "/Game/ArenaAssets/SpellEffects/BP_Effect_PCCleAOEBubble.BP_Effect_PCCleAOEBubble_C" 0 0.0 (.AsArena%20Character (Utilities|Casting|CastToArenaCharacter (Variables|Default|GetInstigator))) self))))

(event Collision|EventActorEndOverlap
  (params (OtherActor :type Actor%20Object%20Reference))
  (Networking|SwitchHasAuthority
    (:Authority
      (bind _asarena_character (Utilities|Casting|CastToArenaCharacter OtherActor))
      (Default|DispelEventbyLogic _asarena_character self true))))

(fn ConstructionScript
  (|CallParentFunction))

(fn HandleDamage
  (params (Damage :type Float%20%28single-precision%29))
  (LocalVariables|SetTempAmount Damage)
  (Utilities|FlowControl|Sequence
    (:then_0
      (if (>= (LocalVariables|GetTempAmount) (Variables|Default|GetSpecialDamageVar))
        (LocalVariables|SetTempAmount (- (LocalVariables|GetTempAmount) (Variables|Default|GetSpecialDamageVar)))
        (Variables|Default|SetSpecialDamageVar 0.0)
        (else
          (LocalVariables|SetTempAmount 0.0)
          (Variables|Default|SetSpecialDamageVar (- (Variables|Default|GetSpecialDamageVar) (LocalVariables|GetTempAmount))))))
    (:then_1
      (if (<= (Variables|Default|GetSpecialDamageVar) 0.0)
        (CallFunction|DestroyLogic)))
    (:then_2
      (return (LocalVariables|GetTempAmount)))))