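; BP_PCFrostbolt is a frostbolt spell projectile that damages non-friendly characters it overlaps.
; When its ProjectileSphere begins an overlap, it checks friendliness, calls CalculateDamage, then passes a hardcoded damage amount to the ArenaCharacter's HandleDamageServer.
; The call to CalculateDamage does not feed that amount.
; DestroyLogic runs after the hit; these helper functions are defined outside this graph.
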(event `self.ReceiveBeginPlay`
  (`parent.ReceiveBeginPlay`))

(event `self.ReceiveActorBeginOverlap`
  (params (OtherActor :type "Actor Object Reference")))

(event `self.ReceiveTick`
  (params (DeltaSeconds :type "Float (single-precision)")))

(event `self.ProjectileSphere.OnComponentBeginOverlap`
  (params (OtherActor :type "Actor Object Reference") (OtherComp :type "PrimitiveComponent Object Reference") (OtherBodyIndex :type Integer) (bFromSweep :type Boolean) (SweepResult :type "HitResult Structure (by ref)"))
  (bind (_success _friendly) (`self.IsFriendly` OtherActor))
  (if (and _success (not _friendly))
    (`self.CalculateDamage` self)
    (`/Game/ArenaAssets/ArenaCharacter.HandleDamage_Server` (cast `/Game/ArenaAssets/ArenaCharacter` OtherActor :!pure true) 500.0 (`self.DamageType`) (`self.GetInstigatorController`) self)
    (`self.DestroyLogic`)))

(fn `UserConstructionScript`
  (`parent.UserConstructionScript`))