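; BP_GenericAutoHit is a generic spell actor that hits its homing target immediately on spawn.
; On BeginPlay it snaps its root to HomingTarget and runs the parent BeginPlay.
; Unless the damage type matches one excluded enum value, it calculates damage and passes it to the target's HandleDamageServer, crediting the instigator controller and itself as causer.
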(event `self.ReceiveBeginPlay`
  (`self.K2_AttachRootComponentToActor` (`self.HomingTarget`) "None" "SnapToTarget")
  (`parent.ReceiveBeginPlay`)
  (if (`|EnumInequality` (`self.DamageType`) "NewEnumerator21")
    (bind _totaldamage (`self.CalculateDamage`))
    (`/Game/ArenaAssets/ArenaCharacter.HandleDamage_Server` (`self.HomingTarget`) _totaldamage (`self.DamageType`) (`self.GetInstigatorController`) self false false)))

(fn `UserConstructionScript`
  (`parent.UserConstructionScript`))