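; Spell logic actor for the Druid's Blessing of the Grove, an aura attached to its homing target with a limited number of heal-over-time activations.
; On spawn it applies the aura effect to that target, then gives overlapping arena characters a Ref effect, dispelled when they leave.
; Each targeted activation applies the HOT effect to the chosen character and spends a charge; the last dispels the aura and destroys the logic.
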(event `self.ReceiveBeginPlay`
  (bind _homingtarget (`self.HomingTarget`))
  (`self.K2_AttachRootComponentToActor` _homingtarget "None" "SnapToTarget")
  (`parent.ReceiveBeginPlay`)
  (`/Game/ArenaAssets/ArenaCharacter.ApplyEffect` _homingtarget "/Game/ArenaAssets/SpellEffects/BP_Effect_PCDruBlessingOfTheGroveAura.BP_Effect_PCDruBlessingOfTheGroveAura_C" 0 0.0 (`self.OwnerPawn`) self))

(event `self.ReceiveActorBeginOverlap`
  (params (OtherActor :type "Actor Object Reference"))
  (bind _asarena_character (cast `/Game/ArenaAssets/ArenaCharacter` OtherActor))
  (`/Game/ArenaAssets/ArenaCharacter.ApplyEffect` _asarena_character "/Game/ArenaAssets/SpellEffects/BP_Effect_PCDruBlessingOfTheGroveRef.BP_Effect_PCDruBlessingOfTheGroveRef_C" 0 0.0 (`self.OwnerPawn`) self))

(event `self.ReceiveActorEndOverlap`
  (params (OtherActor :type "Actor Object Reference"))
  (bind _asarena_character (cast `/Game/ArenaAssets/ArenaCharacter` OtherActor))
  (`/Game/ArenaAssets/ArenaCharacter.DispelEventByLogic` _asarena_character self true))

(event `self.TargetedActivation`
  (params (`Target Char` :type "/Game/ArenaAssets/ArenaCharacter Object Reference"))
  (`/Game/ArenaAssets/ArenaCharacter.ApplyEffect` `Target Char` "/Game/ArenaAssets/SpellEffects/BP_Effect_PCDruBlessingOfTheGroveHOT.BP_Effect_PCDruBlessingOfTheGroveHOT_C" 0 0.0 (`self.OwnerPawn`) self)
  (bind _output_get (set `self.ActivationsRemaining` (- (`self.ActivationsRemaining`) 1)))
  (if (<= _output_get 0)
    (`/Game/ArenaAssets/SpellEffects/SpellEffect.Dispel` (`self.AuraReference`))
    (`self.DestroyLogic`)))

(event `self.NextTick`)

(fn `UserConstructionScript`
  (`parent.UserConstructionScript`))