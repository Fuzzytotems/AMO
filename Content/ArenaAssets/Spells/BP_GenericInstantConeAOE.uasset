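; BP_GenericInstantConeAOE is a generic instant cone area-of-effect spell actor that damages enemies in a single pulse.
; Shortly after BeginPlay, a brief delay precedes ActivatePulse, which loops over the Enemies array.
; Each entry is cast to ArenaCharacter and receives freshly calculated damage through HandleDamageServer, credited to the instigator controller with the spell as damage causer.
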(event `self.ReceiveBeginPlay`
  (`parent.ReceiveBeginPlay`)
  (`KismetSystemLibrary.Delay` 0.04)
  (`self.ActivatePulse`))

(event `self.ReceiveActorBeginOverlap`
  (params (OtherActor :type "Actor Object Reference")))

(event `self.ReceiveTick`
  (params (DeltaSeconds :type "Float (single-precision)")))

(event `self.ActivatePulse`
  (for _array_element (`self.Enemies`)
    (bind _totaldamage (`self.CalculateDamage`))
    (`/Game/ArenaAssets/ArenaCharacter.HandleDamage_Server` (cast `/Game/ArenaAssets/ArenaCharacter` _array_element :!pure true) _totaldamage (`self.DamageType`) (`self.GetInstigatorController`) self false false)))

(fn `UserConstructionScript`
  (`parent.UserConstructionScript`))