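; Druid Tranquility spell actor that applies the Tranquility effect to friendly characters on each pulse.
; On BeginPlay it snaps onto its owner pawn so it follows the caster.
; ActivatePulse runs an unstable sort on Friendlies, then applies BP_Effect_Tranquility to up to the first six ArenaCharacters, passing the instigator and itself as spell logic.
; The sort criterion is not defined in this Blueprint.
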(event `self.ReceiveBeginPlay`
  (`parent.ReceiveBeginPlay`)
  (`self.K2_AttachRootComponentToActor` (`self.OwnerPawn`) "None" "SnapToTarget"))

(event `self.ActivatePulse`
  (bind _output (`FuzzytotemsAugmenterBPLibrary.TArraySortObject` (`self.Friendlies`) "EST_UnstableSort"))
  (for _index (range 6)
    (bind _asarena_character (cast `/Game/ArenaAssets/ArenaCharacter` (`KismetArrayLibrary.Array_Get` _output _index)))
    (`/Game/ArenaAssets/ArenaCharacter.ApplyEffect` _asarena_character "/Game/ArenaAssets/SpellEffects/BP_Effect_Tranquility.BP_Effect_Tranquility_C" 0 0.0 (cast `/Game/ArenaAssets/ArenaCharacter` (`self.Instigator`) :!pure true) self)))

(fn `UserConstructionScript`
  (`parent.UserConstructionScript`))