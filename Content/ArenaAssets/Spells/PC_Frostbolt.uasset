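; Frostbolt spell actor that damages the first non-friendly actor it touches.
; On sphere overlap it runs a friendliness check and ignores friendly actors or failed checks.
; For a hostile target it applies calculated damage, credited to the instigator's controller, then destroys itself.
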(event `self.ReceiveBeginPlay`
  (`parent.ReceiveBeginPlay`))

(event `self.ReceiveActorBeginOverlap`
  (params (OtherActor :type "Actor Object Reference")))

(event `self.ReceiveTick`
  (params (DeltaSeconds :type "Float (single-precision)")))

(event `self.Sphere.OnComponentBeginOverlap`
  (params (OtherActor :type "Actor Object Reference") (OtherComp :type "PrimitiveComponent Object Reference") (OtherBodyIndex :type Integer) (bFromSweep :type Boolean) (SweepResult :type "HitResult Structure (by ref)"))
  (bind (_success _friendly) (`self.IsFriendly` OtherActor))
  (if _success
    (if (not _friendly)
      (bind _totaldamage (`self.CalculateDamage` self))
      (`GameplayStatics.ApplyDamage` OtherActor _totaldamage (`self.GetInstigatorController`) self)
      (`self.K2_DestroyActor`))))

(fn `UserConstructionScript`
  (`parent.UserConstructionScript`))