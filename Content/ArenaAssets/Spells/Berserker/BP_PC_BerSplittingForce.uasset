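; Berserker Splitting Force spell actor that deals a single pulse of damage to enemies.
; On BeginPlay it runs the parent logic, waits a brief delay, then calls ActivatePulse.
; The pulse loops over the Enemies array, computes damage per target and sends it through ArenaCharacter's HandleDamageServer, crediting the instigator controller with this actor as damage causer.
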(event `self.ReceiveBeginPlay`
  (`parent.ReceiveBeginPlay`)
  (`KismetSystemLibrary.Delay` 0.03)
  (`self.ActivatePulse`))

(event `self.ActivatePulse`
  (for _array_element (`self.Enemies`)
    (bind _totaldamage (`self.CalculateDamage`))
    (`/Game/ArenaAssets/ArenaCharacter.HandleDamage_Server` (cast `/Game/ArenaAssets/ArenaCharacter` _array_element :!pure true) _totaldamage (`self.DamageType`) (`self.GetInstigatorController`) self false false)))

(fn `UserConstructionScript`
  (`parent.UserConstructionScript`))