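; Spell logic actor, apparently a base, that drives homing, timed pulses, damage and faction checks for arena spells.
; On BeginPlay it loads its data table row and starts a looping timer, with intervals set by casting type and shortened by a caster stat.
; Each server tick fires the empty ActivatePulse event, destroying the actor when activations run out.
; Damage rolls within a SQLite-queried range, scaled by power and charge.
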(event Custom|Set%20Homing%20Target
  (params (HomingTarget :type Arena%20Character%20Object%20Reference))
  (Utilities|IsValid HomingTarget
    (:Is%20Valid
      (Networking|SwitchHasAuthority
        (:Authority
          (Variables|/Script/Engine.ProjectileMovementComponent|SetHomingTargetComponent (Variables|Default|GetProjectileMovement) (Variables|/Game/ArenaAssets/ArenaCharacter.ArenaCharacter_C|GetBillboard HomingTarget)))))))

(event Custom|ActivatePulse)

(event Custom|DestroyLogic
  (Networking|SwitchHasAuthority
    (:Authority
      (Actor|DestroyActor))))

(event EventBeginPlay
  (bind _returnvalue (Utilities|GetDataTableRow "/Game/ArenaAssets/SpellDataTable.SpellDataTable" (Variables|Default|GetSpellIndexName))
    (:then
      (Variables|Default|SetStatStruct _returnvalue)
      (if (Utilities|IsValid (Variables|Default|GetHomingTarget))
        (CallFunction|SetHomingTarget (Variables|Default|GetHomingTarget)))
      (Variables|Default|SetBaseTimeBetweenTicks (Utilities|Select :Index (.CastingType (Utilities|Struct|BreakSpellInfoStruct (Variables|Default|GetStatStruct))) :CT_Cast (|(LogicLifetime/ChannelProcCount) (.BaseLogicLifetime (Utilities|Struct|BreakSpellInfoStruct (Variables|Default|GetStatStruct))) (Math|Conversions|ToFloat(Integer) (.BaseChannelProcCount (Utilities|Struct|BreakSpellInfoStruct (Variables|Default|GetStatStruct))))) :CT_Channeled (|(CastTime/ChannelProcCount) (.BaseCastTime (Utilities|Struct|BreakSpellInfoStruct (Variables|Default|GetStatStruct))) (Math|Conversions|ToFloat(Integer) (.BaseChannelProcCount (Utilities|Struct|BreakSpellInfoStruct (Variables|Default|GetStatStruct))))) :CT_Charged (|(LogicLifetime/ChannelProcCount) (.BaseLogicLifetime (Utilities|Struct|BreakSpellInfoStruct (Variables|Default|GetStatStruct))) (Math|Conversions|ToFloat(Integer) (.BaseChannelProcCount (Utilities|Struct|BreakSpellInfoStruct (Variables|Default|GetStatStruct)))))))
      (bind _output_get (Variables|Default|SetTimeBetweenTicks (/ (Variables|Default|GetBaseTimeBetweenTicks) (+ (Default|FindRawCalculatedStat (.AsBP%20Arena%20Player%20State (Utilities|Casting|CastToBP_ArenaPlayerState (Variables|/Script/Engine.Pawn|GetPlayerState (Game|GetInstigator)))) "NewEnumerator8") 1.0))))
      (if (> (.BaseChannelProcCount (Utilities|Struct|BreakSpellInfoStruct (Variables|Default|GetStatStruct))) 0)
        (bind _output_get_2 (Variables|Default|SetActivations (Utilities|Select :Index (.CastingType (Utilities|Struct|BreakSpellInfoStruct (Variables|Default|GetStatStruct))) :CT_Cast (Math|Float|Truncate (/ (.BaseLogicLifetime (Utilities|Struct|BreakSpellInfoStruct (Variables|Default|GetStatStruct))) _output_get)) :CT_Channeled (Math|Float|Truncate (/ (.BaseCastTime (Utilities|Struct|BreakSpellInfoStruct (Variables|Default|GetStatStruct))) _output_get)) :CT_Charged (Math|Float|Truncate (/ (.BaseLogicLifetime (Utilities|Struct|BreakSpellInfoStruct (Variables|Default|GetStatStruct))) _output_get)))))
        (Variables|Default|SetActivationsRemaining _output_get_2)
        (bind _returnvalue_2 (Utilities|Time|SetTimerbyFunctionName self "NextTick" (Variables|Default|GetTimeBetweenTicks) true))
        (Variables|Default|SetNextTickHandle _returnvalue_2)))))

(event EventDestroyed
  (Class|KismetSystemLibrary|ClearTimerHandle 0 (Variables|Default|GetNextTickHandle)))

(fn ConstructionScript)

(fn OnRepSpellIndexName)

(fn NextTick
  (Networking|SwitchHasAuthority
    (:Authority
      (CallFunction|ActivatePulse)
      (bind _output_get (Variables|Default|SetActivationsRemaining (- (Variables|Default|GetActivationsRemaining) 1)))
      (if (<= _output_get 0)
        (CallFunction|DestroyLogic)))))

(fn CalculateDamage
  (Networking|SwitchHasAuthority
    (:Authority
      (bind (_mindamage _maxdamage) (CallFunction|RetrieveDamageRange))
      (return (Math|Conversions|ToFloat(Integer) (Math|Float|Truncate (* (* (Math|Random|RandomFloatinRange _mindamage _maxdamage) (+ (Variables|Default|GetPowerModifier) 1.0)) (Variables|Default|GetChargePercentile))))))))

(fn RetrieveDamageRange
  (bind _returnvalue (Class|SQLiteDatabase|IsDatabaseRegistered "GameDB"))
  (if _returnvalue
    _
    (else
      (Class|SQLiteDatabase|RegisterDatabase "GameDB" "Content\\ArenaAssets\\Delete_Me_Database\\GameDB.db" true)))
  (bind _returnvalue_2 (Class|SQLiteDatabase|GetDataBP (Utilities|Struct|MakeSQLiteDatabaseReference "GameDB" (Utilities|Array|MakeArray "SpellDataTable")) (Utilities|Array|MakeArray "MinDamage" "MaxDamage") (Class|SQLiteBlueprintFunctionLibrary|QueryFinal (Class|SQLiteBlueprintFunctionLibrary|QueryEnd (Class|SQLiteBlueprintFunctionLibrary|QueryTerm (Class|SQLiteBlueprintFunctionLibrary|QueryStart) "SpellID" "=" (.LookupID (Utilities|Struct|BreakSpellInfoStruct (Variables|Default|GetStatStruct)))))) -1))
  (for _array_element (.ResultRows (Utilities|Struct|BreakSQLiteQueryResult _returnvalue_2))
    (for _array_element_2 (Utilities|Struct|BreakSQLiteQueryResultRow _array_element)
      (Utilities|FlowControl|FlipFlop
        (:A
          (LocalVariables|SetLocalMinDamage (Math|Conversions|ToFloat(Integer) (.Value (Utilities|Struct|BreakSQLiteKeyValuePair _array_element_2)))))
        (:B
          (LocalVariables|SetLocalMaxDamage (Math|Conversions|ToFloat(Integer) (.Value (Utilities|Struct|BreakSQLiteKeyValuePair _array_element_2))))))))
  (return (LocalVariables|GetLocalMinDamage) (LocalVariables|GetLocalMaxDamage)))

(fn IsFriendly
  (params (Target :type Actor%20Object%20Reference))
  (bind _asarena_character (Utilities|Casting|CastToArenaCharacter Target)
    (:then
      (LocalVariables|SetLocalFriendly (== (Variables|/Game/ArenaAssets/ArenaCharacter.ArenaCharacter_C|GetFaction _asarena_character) (Variables|/Game/ArenaAssets/ArenaCharacter.ArenaCharacter_C|GetFaction (.AsArena%20Character (Utilities|Casting|CastToArenaCharacter (Game|GetInstigator)))))))
    (:CastFailed
      (LocalVariables|SetLocalSuccess false)))
  (return (LocalVariables|GetLocalSuccess) (LocalVariables|GetLocalFriendly)))