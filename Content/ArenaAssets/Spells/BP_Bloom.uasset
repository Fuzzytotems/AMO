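; Bloom spell actor that applies an instant hit to its homing target as soon as it spawns.
; On BeginPlay it snaps its root onto the target, runs the parent logic, then passes the calculated damage to the target's server damage handler, crediting the instigator's controller.
; It stays attached for a short delay before calling the destroy logic, with no travel or collision handling of its own.
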(event `self.ReceiveBeginPlay`
  (`self.K2_AttachRootComponentToActor` (`self.HomingTarget`) "None" "SnapToTarget")
  (`parent.ReceiveBeginPlay`)
  (bind _totaldamage (`self.CalculateDamage`))
  (`/Game/ArenaAssets/ArenaCharacter.HandleDamage_Server` (`self.HomingTarget`) _totaldamage "NewEnumerator0" (`self.GetInstigatorController`) self)
  (`KismetSystemLibrary.Delay` 2.5)
  (`self.DestroyLogic`))

(fn `UserConstructionScript`
  (`parent.UserConstructionScript`))