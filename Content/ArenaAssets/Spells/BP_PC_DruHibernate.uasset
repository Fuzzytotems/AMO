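; BP_PC_DruHibernate is the spell logic for the Druid Hibernate spell, acting on its homing target as soon as it begins play.
; After the parent BeginPlay, it checks whether the target is friendly and does nothing more if that check fails.
; Friendly targets receive the friend variant of the Hibernate effect, while others get an ApplyEffect call with no effect specified.
; Both calls pass the owner pawn as instigator and this spell as logic.
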(event `self.ReceiveBeginPlay`
  (`parent.ReceiveBeginPlay`)
  (bind (_success _friendly) (`self.IsFriendly` (`self.HomingTarget`)))
  (if _success
    (if _friendly
      (`/Game/ArenaAssets/ArenaCharacter.ApplyEffect` (`self.HomingTarget`) "/Game/ArenaAssets/SpellEffects/BP_Effect_PCDruHibernateFriend.BP_Effect_PCDruHibernateFriend_C" 0 0.0 (`self.OwnerPawn`) self)
      (else
        (`/Game/ArenaAssets/ArenaCharacter.ApplyEffect` (`self.HomingTarget`) null 0 0.0 (`self.OwnerPawn`) self)))))

(fn `UserConstructionScript`
  (`parent.UserConstructionScript`))