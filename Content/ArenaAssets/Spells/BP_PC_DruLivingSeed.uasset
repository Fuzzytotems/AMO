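; Spell logic for the player Druid's Living Seed, an effect that jumps between friendly characters.
; It applies the Living Seed effect to its homing target on spawn, while overlap events maintain a list of nearby friendlies.
; On Reenable it sorts that list and moves to the first entry if injured, otherwise destroying itself.
; Each jump reapplies the effect with accumulated elapsed ticks as starting stacks and carries over the diminished-effect modifier.
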(event `self.ReceiveBeginPlay`
  (`parent.ReceiveBeginPlay`)
  (`/Game/ArenaAssets/ArenaCharacter.ApplyEffect` (`self.HomingTarget`) "/Game/ArenaAssets/SpellEffects/BP_Effect_PCDruLivingSeed.BP_Effect_PCDruLivingSeed_C" 0 0.0 (`self.OwnerPawn`) self))

(event `self.Reenable`
  (bind _aurareference (`self.AuraReference`))
  (set `self.SpecialDamageVar` (+ (- (`/Game/ArenaAssets/SpellEffects/SpellEffect.Ticks` _aurareference) (`/Game/ArenaAssets/SpellEffects/SpellEffect.TicksRemaining` _aurareference)) (`self.SpecialDamageVar`)))
  (`self.DetachRootComponentFromParent` true)
  (bind _output (`FuzzytotemsAugmenterBPLibrary.TArraySortObject` (`self.Friendlies`) "EST_Sort"))
  (bind _asarena_character (cast `/Game/ArenaAssets/ArenaCharacter` (`KismetArrayLibrary.Array_Get` _output)))
  (if (< (`/Game/ArenaAssets/ArenaCharacter.GetHPPercentage` _asarena_character) 1.0)
    (`/Game/ArenaAssets/ArenaCharacter.ApplyEffect` _asarena_character "/Game/ArenaAssets/SpellEffects/BP_Effect_PCDruLivingSeed.BP_Effect_PCDruLivingSeed_C" (`KismetMathLibrary.FTrunc` (`self.SpecialDamageVar`)) (`/Game/ArenaAssets/SpellEffects/SpellEffect.DiminishedEffectModifier` (`self.AuraReference`)) (`self.OwnerPawn`) self)
    (`self.K2_AttachRootComponentToActor` _asarena_character "None" "SnapToTarget")
    (else
      (`self.DestroyLogic`))))

(event `self.ReceiveActorBeginOverlap`
  (params (OtherActor :type "Actor Object Reference"))
  (bind (_success _friendly) (`self.IsFriendly` OtherActor))
  (if (and _success _friendly)
    (`KismetArrayLibrary.Array_AddUnique` (`self.Friendlies`) OtherActor)))

(event `self.ReceiveActorEndOverlap`
  (params (OtherActor :type "Actor Object Reference"))
  (`KismetArrayLibrary.Array_RemoveItem` (`self.Friendlies`) OtherActor))

(fn `UserConstructionScript`
  (`parent.UserConstructionScript`))