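; PC_FlameJet is a flame jet spell actor that damages enemy characters inside its capsule.
; On BeginPlay it snaps its root component onto its instigator, so the jet stays attached to the caster.
; Each server pulse finds overlapping ArenaCharacters, skips friendlies or failed team checks, and applies calculated damage through HandleDamageServer, credited to the instigator's controller.
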(event `self.ReceiveBeginPlay`
  (`parent.ReceiveBeginPlay`)
  (`self.K2_AttachRootComponentToActor` (`self.GetInstigator`) "None" "SnapToTarget"))

(event `self.ReceiveActorBeginOverlap`
  (params (OtherActor :type "Actor Object Reference")))

(event `self.ReceiveTick`
  (params (DeltaSeconds :type "Float (single-precision)")))

(event `self.ActivatePulse_Server`
  (for _array_element (`PrimitiveComponent.GetOverlappingActors` (`self.Capsule`) "/Game/ArenaAssets/ArenaCharacter.ArenaCharacter_C")
    (bind (_success _friendly) (`self.IsFriendly` _array_element))
    (if (and _success (not _friendly))
      (bind _totaldamage (`self.CalculateDamage`))
      (`/Game/ArenaAssets/ArenaCharacter.HandleDamage_Server` (cast `/Game/ArenaAssets/ArenaCharacter` _array_element :!pure true) _totaldamage (`self.DamageType`) (`self.GetInstigatorController`) self))))

(fn `UserConstructionScript`
  (`parent.UserConstructionScript`))