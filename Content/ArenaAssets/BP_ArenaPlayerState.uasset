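; Arena player state that holds a player's stats, damage modifiers, spell-school lockouts and EXP, with most changes restricted to authority.
; Modifier changes set a dirty flag, and Tick then rebuilds calculated stats as base plus additive modifiers, times scalars.
; Removals re-add negated values, and damage modifiers and lockouts are arrays indexed by enum.
; BeginPlay reads the level's EXP threshold from a data table; EXP gains only accumulate.
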(event Custom|UpdateLockouts
  (params (DeltaTime :type Float%20%28single-precision%29))
  (bind _lockouts (Variables|Default|GetLockouts))
  (for _array_element _lockouts
    (if (<= (.TimeRemaining (Utilities|Struct|BreakLockoutStruct _array_element)) 0.0)
      (Utilities|Array|SetArrayElem _lockouts (Math|Conversions|ToInteger(Byte) (.School (Utilities|Struct|BreakLockoutStruct _array_element))) (Utilities|Struct|MakeLockoutStruct (.School (Utilities|Struct|BreakLockoutStruct _array_element)) (Math|Float|Clamp(Float) (- (.TimeRemaining (Utilities|Struct|BreakLockoutStruct _array_element)) DeltaTime) 0.0 6e+01))))))

(event Custom|AddRandomLockoutServer
  (params (NewLockout :type Lockout%20Struct%20Structure))
  (Networking|SwitchHasAuthority
    (:Authority
      (CallFunction|AddLockout NewLockout))))

(event Custom|GainEXP_Local
  (params (EXPGained :type Integer))
  (Networking|SwitchHasAuthority
    (:Authority
      (CallFunction|GainEXPServer EXPGained))))

(event Custom|GainEXP_Server
  (params (EXPGained :type Integer))
  (Networking|SwitchHasAuthority
    (:Authority
      (Variables|Default|SetCurrentEXP (+ EXPGained (Variables|Default|GetCurrentEXP))))))

(event Custom|ServerSideRecalculate
  (Networking|SwitchHasAuthority
    (:Authority
      (CallFunction|RecalculateStats))))

(event EventBeginPlay
  (CallFunction|RecalculateStats)
  (bind _returnvalue (Utilities|GetDataTableRow "/Game/ArenaAssets/EXPInfo/EXPDataTable.EXPDataTable" (Utilities|String|StringToName (Utilities|String|ToString(Integer) (Variables|Default|GetLevel))))
    (:then
      (Variables|Default|SetEXPToLevel (Utilities|Struct|BreakExpStruct _returnvalue)))))

(event EventTick
  (params (DeltaSeconds :type Float%20%28single-precision%29))
  (if (Variables|Default|GetNeedsRecalculated)
    (CallFunction|ServerSideRecalculate))
  (CallFunction|UpdateLockouts DeltaSeconds))

(fn ConstructionScript)

(fn FindDamageModifier
  (params (IsIncoming :type Boolean) (DamageType :type EDamageTypes%20Enum))
  (Networking|SwitchHasAuthority
    (:Authority
      (if IsIncoming
        (LocalVariables|SettempDamageModifier (Variables|Default|GetIncomingDamageModifiers))
        (else
          (LocalVariables|SettempDamageModifier (Variables|Default|GetOutgoingDamageModifiers))))
      (if (<= DamageType (Math|Conversions|ToByte(Integer) (Utilities|Array|Length (LocalVariables|GettempDamageModifier))))
        (LocalVariables|SetDamageModifier (.ModificationAmount (Utilities|Struct|BreakDamageModifierStruct (Utilities|Array|Get(acopy) (LocalVariables|GettempDamageModifier) (Math|Conversions|ToInteger(Byte) DamageType))))))
      (return (LocalVariables|GetDamageModifier)))))

(fn AddDamageModifier
  (params (IsIncoming :type Boolean) (NewDamageModifier :type Damage%20Modifier%20Struct%20Structure))
  (LocalVariables|SettempDamModifier NewDamageModifier)
  (if IsIncoming
    (LocalVariables|SettempDamageModifiers (Variables|Default|GetIncomingDamageModifiers))
    (else
      (LocalVariables|SettempDamageModifiers (Variables|Default|GetOutgoingDamageModifiers))))
  (Utilities|Array|SetArrayElem (LocalVariables|GettempDamageModifiers) (Math|Conversions|ToInteger(Byte) (.DamageType (Utilities|Struct|BreakDamageModifierStruct (Utilities|Array|Get(acopy) (LocalVariables|GettempDamageModifiers) (Math|Conversions|ToInteger(Byte) (.DamageType (Utilities|Struct|BreakDamageModifierStruct (LocalVariables|GettempDamModifier)))))))) (Utilities|Struct|MakeDamageModifierStruct (.DamageType (Utilities|Struct|BreakDamageModifierStruct (Utilities|Array|Get(acopy) (LocalVariables|GettempDamageModifiers) (Math|Conversions|ToInteger(Byte) (.DamageType (Utilities|Struct|BreakDamageModifierStruct (LocalVariables|GettempDamModifier))))))) (+ (.ModificationAmount (Utilities|Struct|BreakDamageModifierStruct (LocalVariables|GettempDamModifier))) (.ModificationAmount (Utilities|Struct|BreakDamageModifierStruct (Utilities|Array|Get(acopy) (LocalVariables|GettempDamageModifiers) (Math|Conversions|ToInteger(Byte) (.DamageType (Utilities|Struct|BreakDamageModifierStruct (LocalVariables|GettempDamModifier))))))))))
  (if IsIncoming
    (Variables|Default|SetIncomingDamageModifiers (LocalVariables|GettempDamageModifiers))
    (else
      (Variables|Default|SetOutgoingDamageModifiers (LocalVariables|GettempDamageModifiers))))
  (Variables|Default|SetNeedsRecalculated true))

(fn AddStatModifier
  (params (NewStatModifier :type Stat%20Struct%20Structure))
  (bind _statmodifiers (Variables|CalculatedStats|GetStatModifiers))
  (Networking|SwitchHasAuthority
    (:Authority
      (bind _output_get (LocalVariables|SettempStatMod NewStatModifier))
      (bind (_array_element _array_index) (Utilities|Array|ForEachLoopwithBreak _statmodifiers :!label _label)
        (:LoopBody
          (if (== (.StatToEffect (Utilities|Struct|BreakStatStruct _output_get)) (.StatToEffect (Utilities|Struct|BreakStatStruct _array_element)))
            (LocalVariables|SettempStatMod (Utilities|Struct|MakeStatStruct (.StatToEffect (Utilities|Struct|BreakStatStruct _array_element)) (+ (.CurrentRating (Utilities|Struct|BreakStatStruct _array_element)) (.CurrentRating (Utilities|Struct|BreakStatStruct _output_get)))))
            (Utilities|Array|RemoveIndex _statmodifiers _array_index)
            (goto _label Break)))
        (:Completed
          (Utilities|Array|Add _statmodifiers (LocalVariables|GettempStatMod))
          (Variables|Default|SetNeedsRecalculated true))))))

(fn RecalculateStats
  (Networking|SwitchHasAuthority
    (:Authority
      (Utilities|FlowControl|Sequence
        (:then_0
          (LocalVariables|SetTempCalculatedStats (Variables|BaseStats|GetBaseStats)))
        (:then_1
          (bind _array_element (Utilities|Array|ForEachLoopwithBreak (Variables|CalculatedStats|GetStatModifiers))
            (:LoopBody
              (Utilities|Array|SetArrayElem (LocalVariables|GetTempCalculatedStats) (Math|Conversions|ToInteger(Byte) (.StatToEffect (Utilities|Struct|BreakStatStruct _array_element))) (Utilities|Struct|MakeStatStruct (.StatToEffect (Utilities|Struct|BreakStatStruct (Utilities|Array|Get(acopy) (LocalVariables|GetTempCalculatedStats) (Math|Conversions|ToInteger(Byte) (.StatToEffect (Utilities|Struct|BreakStatStruct _array_element)))))) (+ (.CurrentRating (Utilities|Struct|BreakStatStruct _array_element)) (.CurrentRating (Utilities|Struct|BreakStatStruct (Utilities|Array|Get(acopy) (LocalVariables|GetTempCalculatedStats) (Math|Conversions|ToInteger(Byte) (.StatToEffect (Utilities|Struct|BreakStatStruct _array_element))))))))))))
        (:then_2
          (bind _array_element_2 (Utilities|Array|ForEachLoopwithBreak (Variables|CalculatedStats|GetStatScalars))
            (:LoopBody
              (Utilities|Array|SetArrayElem (LocalVariables|GetTempCalculatedStats) (Math|Conversions|ToInteger(Byte) (.StatToEffect (Utilities|Struct|BreakStatStruct _array_element_2))) (Utilities|Struct|MakeStatStruct (.StatToEffect (Utilities|Struct|BreakStatStruct (Utilities|Array|Get(acopy) (LocalVariables|GetTempCalculatedStats) (Math|Conversions|ToInteger(Byte) (.StatToEffect (Utilities|Struct|BreakStatStruct _array_element_2)))))) (* (.CurrentRating (Utilities|Struct|BreakStatStruct _array_element_2)) (.CurrentRating (Utilities|Struct|BreakStatStruct (Utilities|Array|Get(acopy) (LocalVariables|GetTempCalculatedStats) (Math|Conversions|ToInteger(Byte) (.StatToEffect (Utilities|Struct|BreakStatStruct _array_element_2))))))))))
            (:Completed
              (Variables|Default|SetNeedsRecalculated false)
              (Variables|CalculatedStats|SetCalculatedStats (LocalVariables|GetTempCalculatedStats)))))))))

(fn RemoveDamageModifier
  (params (IsIncoming :type Boolean) (RemovedDamageModifier :type Damage%20Modifier%20Struct%20Structure))
  (bind (_damagetype _modificationamount) (Utilities|Struct|BreakDamageModifierStruct RemovedDamageModifier))
  (CallFunction|AddDamageModifier IsIncoming (Utilities|Struct|MakeDamageModifierStruct _damagetype (* _modificationamount -1.0))))

(fn RemoveStatModifier
  (params (NewStatModifier :type Stat%20Struct%20Structure))
  (bind (_stattoeffect _currentrating) (Utilities|Struct|BreakStatStruct NewStatModifier))
  (CallFunction|AddStatModifier (Utilities|Struct|MakeStatStruct _stattoeffect (* _currentrating -1.0))))

(fn AddStatScalar
  (params (TempStatStruct :type Stat%20Struct%20Structure))
  (bind _statscalars (Variables|CalculatedStats|GetStatScalars))
  (Networking|SwitchHasAuthority
    (:Authority
      (bind _output_get (LocalVariables|SetTempStatScalar TempStatStruct))
      (bind (_array_element _array_index) (Utilities|Array|ForEachLoopwithBreak _statscalars :!label _label)
        (:LoopBody
          (if (== (.StatToEffect (Utilities|Struct|BreakStatStruct _output_get)) (.StatToEffect (Utilities|Struct|BreakStatStruct _array_element)))
            (LocalVariables|SetTempStatScalar (Utilities|Struct|MakeStatStruct (.StatToEffect (Utilities|Struct|BreakStatStruct _array_element)) (+ (.CurrentRating (Utilities|Struct|BreakStatStruct _output_get)) (.CurrentRating (Utilities|Struct|BreakStatStruct _array_element)))))
            (Utilities|Array|RemoveIndex _statscalars _array_index)
            (goto _label Break)))
        (:Completed
          (Utilities|Array|Add _statscalars (LocalVariables|GetTempStatScalar))
          (Variables|Default|SetNeedsRecalculated true))))))

(fn RemoveStatScalar
  (params (TempStatStruct :type Stat%20Struct%20Structure))
  (bind (_stattoeffect _currentrating) (Utilities|Struct|BreakStatStruct TempStatStruct))
  (CallFunction|AddStatScalar (Utilities|Struct|MakeStatStruct _stattoeffect (* _currentrating -1.0))))

(fn FindRawCalculatedStat
  (params (RawStatToFind :type EStatToEffect%20Enum))
  (return (.CurrentRating (Utilities|Struct|BreakStatStruct (Utilities|Array|Get(acopy) (Variables|CalculatedStats|GetCalculatedStats) (Math|Conversions|ToInteger(Byte) RawStatToFind))))))

(fn FindCalculatedStat)

(fn AddLockout
  (params (NewLockout :type Lockout%20Struct%20Structure))
  (Networking|SwitchHasAuthority
    (:Authority
      (Utilities|Array|SetArrayElem (Variables|Default|GetLockouts) (Math|Conversions|ToInteger(Byte) (.School (Utilities|Struct|BreakLockoutStruct NewLockout))) NewLockout))))