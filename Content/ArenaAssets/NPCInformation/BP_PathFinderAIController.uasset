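; AI controller for path-following arena NPCs that tracks hostile characters and drives a behavior tree.
; On BeginPlay it retries until it controls an AICharacter, then runs the tree and seeds the blackboard with the pawn's desired path node.
; Perception updates filter out same-faction characters, maintain an enemy list and set the enemy-visible key.
; Helpers set the blackboard enemy and forward spell casting and targeting to the pawn.
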(event OnPerceptionUpdated(AIPerception)
  (params (UpdatedActors :type Array%20of%20Actor%20Object%20References))
  (for _array_element UpdatedActors
    (bind _info (Class|AIPerceptionComponent|GetActorsPerception (Variables|Default|GetAIPerception) _array_element))
    (bind _asarena_character (Utilities|Casting|CastToArenaCharacter _array_element))
    (bind _friendly (CallFunction|IsFriendly _asarena_character))
    (if (not _friendly)
      (CallFunction|AddNewEnemy _asarena_character (.bSuccessfullySensed (Utilities|Struct|BreakAIStimulus (Utilities|Array|Get(acopy) (.LastSensedStimuli (Utilities|Struct|BreakActorPerceptionBlueprintInfo _info))))))
      (AI|Components|Blackboard|SetValueasBool (AI|GetBlackboard 0) (Variables|Default|GetBlackboardKeyEnemyVisible) (> (Utilities|Array|Length (Variables|Default|GetEnemyList)) 0)))))

(event Custom|SetTarget
  (params (NewTarget :type Arena%20Character%20Object%20Reference))
  (Default|FrameSelectTarget (Variables|Default|GetStoredPawn) NewTarget))

(event Custom|CastSpell
  (params (Spell%20Name :type Name))
  (Default|HandleTargetingEvent (Variables|Default|GetStoredPawn) Spell%20Name)
  (Development|PrintString (Utilities|String|ToString(Name) Spell%20Name)))

(event EventBeginPlay
  (bind _asaicharacter (Utilities|Casting|CastToAICharacter (Pawn|GetControlledPawn) :!label _label)
    (:then
      (Actor|Tick|SetActorTickEnabled true)
      (bind _output_get (Variables|Default|SetStoredPawn _asaicharacter))
      (AI|RunBehaviorTree "/Game/ArenaAssets/NPCInformation/PathFollowerBT.PathFollowerBT")
      (AI|Components|Blackboard|SetValueasObject (AI|GetBlackboard 0) (Variables|Default|GetDesiredPathNodeKey) (Variables|/Game/ArenaAssets/NPCInformation/AICharacter.AICharacter_C|GetDesiredNode _output_get)))
    (:CastFailed
      (Utilities|FlowControl|RetriggerableDelay 0.06)
      (goto _label))))

(fn ConstructionScript
  (Variables|Default|SetbWantsPlayerState true))

(fn SetNewEnemy
  (params (Enemy :type Actor%20Object%20Reference))
  (if (!= Enemy (Variables|Default|GetEnemy))
    (bind _output_get (Variables|Default|SetEnemy Enemy))
    (AI|Components|Blackboard|SetValueasObject (AI|GetBlackboard 0) (Variables|Default|GetEnemyKey) _output_get)))

(fn AddNewEnemy
  (params (NewEnemyToAdd :type Actor%20Object%20Reference) (Detected :type Boolean))
  (bind _enemylist (Variables|Default|GetEnemyList))
  (if Detected
    (Utilities|Array|AddUnique _enemylist NewEnemyToAdd)
    (else
      (Utilities|Array|RemoveItem _enemylist NewEnemyToAdd))))

(fn IsFriendly
  (params (Target :type Arena%20Character%20Object%20Reference))
  (LocalVariables|SetLocalFriendly (== (Variables|/Game/ArenaAssets/ArenaCharacter.ArenaCharacter_C|GetFaction Target) (Variables|/Game/ArenaAssets/ArenaCharacter.ArenaCharacter_C|GetFaction (.AsArena%20Character (Utilities|Casting|CastToArenaCharacter (Pawn|GetControlledPawn))))))
  (return (LocalVariables|GetLocalFriendly)))