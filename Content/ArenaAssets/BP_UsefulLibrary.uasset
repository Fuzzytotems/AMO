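; Helper library for the arena spell system, providing a line-of-sight check and spell stat modification.
; CheckOutOfLOS traces against WorldStatic with persistent debug drawing, returning any hit when FrameTargeted, otherwise ignoring hits in the last sliver of the trace.
; AddSpellModifier switches on modifier type, applying nonzero flat reductions or else scalars to numeric fields, appending effects, or setting cast-while-moving.
; FriendFoeStatus is a stub returning zero.
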(fn CheckOutOfLOS
  (params (WorldContextObject :type Actor%20Object%20Reference) (Start :type Vector) (End :type Vector) (FrameTargeted :type Boolean))
  (bind (_outhit _returnvalue) (Collision|LineTraceForObjects WorldContextObject Start End (Utilities|Array|MakeArray "ObjectTypeQuery1") false 0 "Persistent"))
  (if FrameTargeted
    (LocalVariables|SetEndResult _returnvalue)
    (else
      (LocalVariables|SetEndResult (not (> (.Time (Collision|BreakHitResult _outhit)) 0.98)))))
  (return (LocalVariables|GetEndResult)))

(fn FriendFoeStatus
  (return 0.0))

(fn AddSpellModifier
  (params (Spell :type Spell%20Info%20Struct%20Structure) (SpellModifierStruct :type Spell%20Modifier%20Struct%20Structure))
  (bind (_rawspellid _spellname _spelllogic _castingtype _disabletype _aimingtype _playertargetingrules _magicschools _basecasttime _basecastwhilemoving _basecooldown _baselogiclifetime _baseresourcecost _baserange _basechannelproccount _basemaxcharges _cdlinename _cdsalsotriggered _castingparticles_hands _castingparticles_body _castingparticles_feet _positiveeffects _negativeeffects _castingparticles_hands_offset _castingparticles_body_offset _castingparticles_feet_offset _spellicon _targetingscale _damagescaling _resourcecostscaling _baselevel _castanimation _lookupid _isbuilder _isvariablespender _spendingintervals _minimumspend _maximumspend _alternativeresourcespentid _minaltresource _maxaltresource) (Utilities|Struct|BreakSpellInfoStruct Spell))
  (bind (_modifiertype _flatreduction _scalarmodifier _positiveeffects_2 _negativeeffects_2 _castwhilemoving) (Utilities|Struct|BreakSpellModifierStruct SpellModifierStruct))
  (bind _returnvalue (!= _flatreduction 0.0))
  (bind _returnvalue_2 (Math|Float|Truncate _flatreduction))
  (Utilities|FlowControl|Sequence
    (:then_0
      (switch Utilities|FlowControl|Switch|SwitchonSpellModifierEnum _modifiertype
        (:NewEnumerator0
          ;[1 1 1] Cast Time
          (if _returnvalue
            (bind _structout (Utilities|Struct|SetmembersinSpellInfoStruct Spell (- _basecasttime _flatreduction)))
            (LocalVariables|SetResultingSpell _structout)
            (else
              (bind _structout_2 (Utilities|Struct|SetmembersinSpellInfoStruct Spell (* _basecasttime _scalarmodifier)))
              (LocalVariables|SetResultingSpell _structout_2))))
        (:NewEnumerator2
          ;[1 1 1] Cooldown
          (if _returnvalue
            (bind _structout_3 (Utilities|Struct|SetmembersinSpellInfoStruct Spell (- _basecooldown _flatreduction)))
            (LocalVariables|SetResultingSpell _structout_3)
            (else
              (bind _structout_4 (Utilities|Struct|SetmembersinSpellInfoStruct Spell (* _basecooldown _scalarmodifier)))
              (LocalVariables|SetResultingSpell _structout_4))))
        (:NewEnumerator3
          ;[1 1 1] Resource Cost
          (if _returnvalue
            (bind _structout_5 (Utilities|Struct|SetmembersinSpellInfoStruct Spell (- _baseresourcecost _flatreduction)))
            (LocalVariables|SetResultingSpell _structout_5)
            (else
              (bind _structout_6 (Utilities|Struct|SetmembersinSpellInfoStruct Spell (* _baseresourcecost _scalarmodifier)))
              (LocalVariables|SetResultingSpell _structout_6))))
        (:NewEnumerator4
          ;[1 1 1] Charges
          (if _returnvalue
            (bind _structout_7 (Utilities|Struct|SetmembersinSpellInfoStruct Spell (- _basemaxcharges _returnvalue_2)))
            (LocalVariables|SetResultingSpell _structout_7)
            (else
              (bind _structout_8 (Utilities|Struct|SetmembersinSpellInfoStruct Spell (Math|Float|Truncate (* _basemaxcharges _scalarmodifier))))
              (LocalVariables|SetResultingSpell _structout_8))))
        (:NewEnumerator5
          ;[1 1 1] MinimumAltResource
          (if _returnvalue
            (bind _structout_9 (Utilities|Struct|SetmembersinSpellInfoStruct Spell (- _minaltresource _returnvalue_2)))
            (LocalVariables|SetResultingSpell _structout_9)
            (else
              (bind _structout_10 (Utilities|Struct|SetmembersinSpellInfoStruct Spell (Math|Float|Truncate (* _minaltresource _scalarmodifier))))
              (LocalVariables|SetResultingSpell _structout_10))))
        (:NewEnumerator8
          ;[1 1 1] Maximum Alt Resource
          (if _returnvalue
            (bind _structout_11 (Utilities|Struct|SetmembersinSpellInfoStruct Spell (- _maxaltresource _returnvalue_2)))
            (LocalVariables|SetResultingSpell _structout_11)
            (else
              (bind _structout_12 (Utilities|Struct|SetmembersinSpellInfoStruct Spell (Math|Float|Truncate (* _maxaltresource _scalarmodifier))))
              (LocalVariables|SetResultingSpell _structout_12))))
        (:NewEnumerator6
          (bind _output_get (LocalVariables|SetEffectList _positiveeffects))
          (Utilities|Array|Add _output_get _positiveeffects_2)
          (bind _structout_13 (Utilities|Struct|SetmembersinSpellInfoStruct Spell _output_get))
          (LocalVariables|SetResultingSpell _structout_13))
        (:NewEnumerator7
          (bind _output_get_2 (LocalVariables|SetEffectList _negativeeffects))
          (Utilities|Array|Add _output_get_2 _negativeeffects_2)
          (bind _structout_14 (Utilities|Struct|SetmembersinSpellInfoStruct Spell _output_get_2))
          (LocalVariables|SetResultingSpell _structout_14))
        (:NewEnumerator1
          (bind _structout_15 (Utilities|Struct|SetmembersinSpellInfoStruct Spell _castwhilemoving))
          (LocalVariables|SetResultingSpell _structout_15))))
    (:then_1
      (return (LocalVariables|GetResultingSpell)))))